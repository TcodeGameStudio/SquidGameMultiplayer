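; BP_StartedWall is a barrier actor that disappears once the doll signals the game has started.
; On BeginPlay it caches the first BP_Doll in the level.
; Each Tick it polls the doll's IsStart flag and, while the Cube component is still valid, calls DestroyWall to remove that cube.
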(event Custom|DestroyWall
  (Components|DestroyComponent (Variables|Default|GetCube)))

(event EventTick
  (params (DeltaSeconds :type Float%20%28single-precision%29))
  (if (and (Variables|/Game/Blueprints/BP_Doll.BP_Doll_C|GetIsStart (Variables|Default|GetDoll)) (Utilities|IsValid (Variables|Default|GetCube)))
    (CallFunction|DestroyWall)))

(event EventBeginPlay
  (bind _outactors (Actor|GetAllActorsOfClass "/Game/Blueprints/BP_Doll.BP_Doll_C"))
  (Variables|Default|SetDoll (Utilities|Array|Get(acopy) _outactors)))

(fn ConstructionScript)