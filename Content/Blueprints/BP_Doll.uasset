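; Turning doll that alternates head rotation with a sound cue, apparently for a Red Light, Green Light style game.
; While started, Tick drives a FlipFlop: one side waits, flags DirectionBackward and plays a yaw Timeline on the head.
; The other plays audio at a randomized pitch to vary its length, then clears the flag and reverses the Timeline when audio finishes.
; AnimationIsComplete gates each step until the Timeline finishes.
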(event Custom|OnAudioFinished_Event
  (Variables|Default|SetdirectionBackward false)
  (bind _z (Timeline|Timeline Reverse)
    (:Update
      (Transformation|SetRelativeRotation (Variables|Default|GetDollHead) (Math|Rotator|MakeRotator 0.0 0.0 _z) false false))
    (:Finished
      (Variables|Default|SetanimationIsComplete true)
      (Variables|Default|SetFirstDuration 2.0))))

(event Custom|Server%20Doll%20Movement
  (bind _audio (Variables|Default|GetAudio))
  (bind _dollsound (Variables|Components|GetdollSound))
  (bind _duration (Variables|/Script/Engine.SoundBase|GetDuration _dollsound))
  (if (and (Variables|Default|GetIsStart) (Variables|Default|GetanimationIsComplete))
    (Variables|Default|SetanimationIsComplete false)
    (Utilities|FlowControl|FlipFlop
      (:A
        (Utilities|FlowControl|Delay (Variables|Default|GetFirstDuration))
        (Variables|Default|SetdirectionBackward true)
        (bind _z (Timeline|Timeline Play)
          (:Update
            (Transformation|SetRelativeRotation (Variables|Default|GetDollHead) (Math|Rotator|MakeRotator 0.0 0.0 _z) false false))
          (:Finished
            (Variables|Default|SetanimationIsComplete true)
            (Variables|Default|SetFirstDuration 2.0))))
      (:B
        (CallFunction|ServerSound _audio (+ (/ (Math|Random|RandomFloatinRange 2.0 _duration) _duration) 1.0))
        (EventDispatchers|BindEventtoOnAudioFinished _audio (delegate Custom|OnAudioFinished_Event))))))

(event Custom|ServerSound
  (params (Audio :type Audio%20Component%20Object%20Reference) (Duration :type Float%20%28double-precision%29))
  (Audio|Components|Audio|SetPitchMultiplier Audio Duration)
  (Audio|Components|Audio|Play Audio 0.0))

(event EventBeginPlay
  (Variables|Default|SetFirstDuration 0.0))

(event EventTick
  (params (DeltaSeconds :type Float%20%28single-precision%29))
  (CallFunction|ServerDollMovement))

(fn ConstructionScript)